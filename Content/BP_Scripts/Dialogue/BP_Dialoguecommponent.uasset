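; BP_Dialoguecommponent is a dialogue component that shows one line of data-driven dialogue each time its Interact event fires.
; Interact looks up the current row in a DataTable and creates a WB_Dialogue widget with the speaker name and that row's text, then adds it to the viewport.
; It then stores the row's next row name, DataTable and end flag, so entries chain across rows and tables.
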(event `/Game/BP_Scripts/Dialogue/BP_Interact.Interact`
  (params (PlayerRef :type "/Game/BP_Scripts/BP_Character Object Reference"))
  (bind _returnvalue (`|GetDataTableRow` (`self.Data Table`) (`self.Row Name`))
    (:`then`
      (bind (_dialogue _row _datatable _enddialouge_) (break `/Game/BP_Scripts/Dialogue/Dialogue_Structure` _returnvalue))
      (bind _returnvalue_2 (`|CreateWidget` "/Game/BP_Scripts/Dialogue/WB_Dialogue.WB_Dialogue_C" null (`KismetTextLibrary.Conv_NameToText` (`self.Name`)) _dialogue))
      (bind _output_get (set `self.DialogueWidget` _returnvalue_2))
      (`UserWidget.AddToViewport` _output_get 0)
      (set `self.Row Name` _row)
      (set `self.Data Table` _datatable)
      (set `self.EndDialogue` _enddialouge_))))