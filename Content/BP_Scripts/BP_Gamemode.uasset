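; BP_Gamemode is a game mode that scatters fossil dirt mounds at random locations when play begins.
; SpawnFossils gathers every BP_SpawnPoint actor, then loops a fixed few times, spawning a BP_Mound at a randomly picked point.
; Each used point is removed from the local list and destroyed so mounds do not share a location.
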(event `self.ReceiveBeginPlay`
  (`self.SpawnFossils`))

(fn `SpawnFossils`
  (locals (LocalSpawnRefrences :type "Array of Actor Object Reference") (`Local item` :type "Actor Object Reference"))
  (bind _local_item (`local.Local item`))
  ;[1 1 1] Actor class is the spawn locations
  (bind _outactors (`GameplayStatics.GetAllActorsOfClass` "/Game/BP_Scripts/BP_SpawnPoint.BP_SpawnPoint_C"))
  (set `local.LocalSpawnRefrences` _outactors)
  ;[1 1 1] Create last index max amount of spawnable items
  (for _ (range 3)
    (set `local.Local item` (`KismetArrayLibrary.Array_Random` (`local.LocalSpawnRefrences`)))
    ;[1 1 1] Class is the actor you want to spawn (Dirt mounds)
    (`|SpawnActorFromClass` "/Game/BP_Scripts/BP_Mound.BP_Mound_C" (`KismetMathLibrary.MakeTransform` (`self.K2_GetActorLocation` (`local.Local item`))) "AdjustIfPossibleButAlwaysSpawn" "MultiplyWithRoot" null null)
    ;[1 1 1] Stops from spawning in the same place
    (`KismetArrayLibrary.Array_RemoveItem` (`local.LocalSpawnRefrences`) _local_item)
    (`self.K2_DestroyActor` _local_item)))

(fn `UserConstructionScript`)