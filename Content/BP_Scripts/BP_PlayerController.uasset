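; BP_PlayerController is a player controller that handles movement and interaction for the controlled pawn through Enhanced Input.
; BeginPlay adds the input mapping context, and AC_Move feeds its X and Y values into AddMovementInput as a world-space direction.
; When AC_Interact starts, it prints a leftover on-screen string, then sends InteractMessage to the first overlapping actor that implements InteractInterface.
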(event `EnhancedInput|/Game/BP_Scripts/AC_Move`
  (params (ActionValue :type "Vector2D Structure") (ElapsedSeconds :type "Float (double-precision)") (TriggeredSeconds :type "Float (double-precision)") (InputAction :type "InputAction Object Reference" :default "/Game/BP_Scripts/AC_Move.AC_Move"))
  (bind (_x _y) (`KismetMathLibrary.BreakVector2D` ActionValue))
  ;[1 1 1] Movement
  (:`Triggered`
    (`Pawn.AddMovementInput` (`self.K2_GetPawn`) (`KismetMathLibrary.MakeVector` _x _y) 1.0 false)))

(event `EnhancedInput|/Game/BP_Scripts/AC_Interact`
  (params (ActionValue :type "Float (double-precision)") (ElapsedSeconds :type "Float (double-precision)") (TriggeredSeconds :type "Float (double-precision)") (InputAction :type "InputAction Object Reference" :default "/Game/BP_Scripts/AC_Interact.AC_Interact"))
  ;[1 1 1] Interaction
  (:`Started`
    (`KismetSystemLibrary.PrintString` "Chat what should i say to malachi? \nNo I am not going to say \"Kiss me gay boy\"")
    (for _array_element (`self.GetOverlappingActors` (`self.K2_GetPawn`) "/Script/Engine.Actor")
      (if (`KismetSystemLibrary.DoesImplementInterface` _array_element "/Game/BP_Scripts/InteractInterface.InteractInterface_C")
        (message `/Game/BP_Scripts/InteractInterface.Interact` _array_element)
        (break)))))

(event `self.ReceiveBeginPlay`
  ;[1 1 1] Sets up the controller
  (`EnhancedInputSubsystemInterface.AddMappingContext` (subsystem `EnhancedInputLocalPlayerSubsystem`) "/Game/BP_Scripts/InputMapping.InputMapping" 0 (struct)))

(fn `UserConstructionScript`)