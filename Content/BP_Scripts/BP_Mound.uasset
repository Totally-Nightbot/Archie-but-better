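; BP_Mound is an interactable mound that grants Archie, the player, the echidna skull and then disappears.
; Box overlap events track whether the player is inside by comparing display names, though the end-overlap check has no actor input.
; Interact, when InCollider is set, flags Archiegotskull on every BP_EchidnaSkull in the level and destroys the mound from within that loop.
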(event `/Game/BP_Scripts/InteractInterface.Interact`
  ;[1 1 1] Trialing interact
  (if (`self.InCollider`)
    (set `self.InCollider` false)
    (bind _outactors (`GameplayStatics.GetAllActorsOfClass` "/Game/BP_Scripts/BP_EchidnaSkull.BP_EchidnaSkull_C"))
    (for _array_element _outactors
      (set `/Game/BP_Scripts/BP_EchidnaSkull.Archiegotskull` true _array_element)
      (`self.K2_DestroyActor`))))

(event `self.Box.OnComponentBeginOverlap`
  (params (OverlappedComponent :type "PrimitiveComponent Object Reference") (OtherActor :type "Actor Object Reference") (OtherComp :type "PrimitiveComponent Object Reference") (OtherBodyIndex :type Integer) (bFromSweep :type Boolean) (SweepResult :type "HitResult Structure (by ref)"))
  ;[1 1 1] If Overlap, then set to true
  (if (`KismetStringLibrary.EqualEqual_StrStr` (`KismetSystemLibrary.GetDisplayName` OtherActor) (`KismetSystemLibrary.GetDisplayName` (`GameplayStatics.GetPlayerPawn` 0)))
    (set `self.InCollider` true)
    (`KismetSystemLibrary.PrintString` "Archie overlapped")))

(event `self.Box.OnComponentEndOverlap`
  (params (OverlappedComponent :type "PrimitiveComponent Object Reference") (OtherActor :type "Actor Object Reference") (OtherComp :type "PrimitiveComponent Object Reference") (OtherBodyIndex :type Integer))
  ;[1 1 1] if leave overlap set to false
  (if (`KismetStringLibrary.EqualEqual_StrStr` (`KismetSystemLibrary.GetDisplayName` null) (`KismetSystemLibrary.GetDisplayName` (`GameplayStatics.GetPlayerPawn` 0)))
    (set `self.InCollider` false)
    (`KismetSystemLibrary.PrintString` "Archie Leave Overlap")))

(fn `UserConstructionScript`)